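; Random NFT avatar generator that builds a male or female character head when its lever passes a threshold or a player inside its box presses R.
; Random DataTable rows supply the head and, where allowed, hair or hat, eyebrows and male beard, all attached to a head socket.
; Dynamic material instances randomize each part's colors.
; Each reroll, guarded by IsRandom, clears meshes, rebuilds after a delay, then shows mesh names in a result widget.
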(event OnComponentBeginOverlap(Box)
  (params (OverlappedComponent :type Primitive%20Component%20Object%20Reference) (OtherActor :type Actor%20Object%20Reference) (OtherComp :type Primitive%20Component%20Object%20Reference) (OtherBodyIndex :type Integer) (bFromSweep :type Boolean) (SweepResult :type Hit%20Result%20Structure%20%28by%20ref%29))
  (bind _asvoice_chat_character (Utilities|Casting|CastToVoiceChatCharacter OtherActor))
  (bind _as플레이어_컨트롤러 (Utilities|Casting|CastToPlayerController (Pawn|GetController _asvoice_chat_character)))
  (Input|EnableInput _as플레이어_컨트롤러))

(event OnComponentEndOverlap(Box)
  (params (OverlappedComponent :type Primitive%20Component%20Object%20Reference) (OtherActor :type Actor%20Object%20Reference) (OtherComp :type Primitive%20Component%20Object%20Reference) (OtherBodyIndex :type Integer))
  (bind _asvoice_chat_character (Utilities|Casting|CastToVoiceChatCharacter OtherActor))
  (bind _as플레이어_컨트롤러 (Utilities|Casting|CastToPlayerController (Pawn|GetController _asvoice_chat_character)))
  (Input|DisableInput _as플레이어_컨트롤러))

(event Custom|CreateNFT
  (bind _head (Variables|Default|GetHead))
  (bind _head_2 (Variables|Default|GetHead))
  (switch int (Math|Random|RandomIntegerinRange 0 1)
    (:0
      (bind _outrownames (DataTable|GetDataTableRowNames "/Game/Main/RandomNFT/FData/DT_F_Head.DT_F_Head"))
      (bind _returnvalue (Utilities|GetDataTableRow "/Game/Main/RandomNFT/FData/DT_F_Head.DT_F_Head" (Utilities|Array|Get(acopy) _outrownames (Math|Random|RandomIntegerinRange 0 (Utilities|Array|Length _outrownames))))
        (:then
          (Components|SkeletalMesh|SetSkeletalMeshAsset _head_2 (.SkeletalMesh (Utilities|Struct|BreakS_Head _returnvalue)))
          (for _array_element (.MaterialNumber (Utilities|Struct|BreakS_Head _returnvalue))
            (bind _returnvalue_2 (Rendering|Material|CreateDynamicMaterialInstance _head_2 _array_element 0 "None" :!class /Script/Engine.PrimitiveComponent))
            (for _index (range 1 (Utilities|Array|Get(acopy) (.ColorCounts (Utilities|Struct|BreakS_Head _returnvalue)) _array_element))
              (bind _newparam (CallFunction|RandomColor))
              (Rendering|Material|SetVectorParameterValue _returnvalue_2 (Utilities|String|StringToName (Utilities|String|Append "Color " (Utilities|String|ToString(Integer) _index))) _newparam :!class /Script/Engine.MaterialInstanceDynamic)))
          (if (.IsHair (Utilities|Struct|BreakS_Head _returnvalue))
            (switch int (Math|Random|RandomIntegerinRange 0 1)
              (:0
                (CallFunction|CustomMesh "/Game/Main/RandomNFT/FData/DT_F_Hair.DT_F_Hair" (Variables|Default|GetHair)))
              (:1
                (CallFunction|CustomMesh "/Game/Main/RandomNFT/FData/DT_F_Hat.DT_F_Hat" (Variables|Default|GetHair))))
            (CallFunction|CustomMesh "/Game/Main/RandomNFT/FData/DT_F_Eyebrow.DT_F_Eyebrow" (Variables|Default|GetEyebrow))
            (Components|StaticMesh|SetStaticMesh (Variables|Default|GetEyes) "/Game/StylizedModularChar/Meshes/SM_Eyes.SM_Eyes")))))
    (:1
      (bind _outrownames_2 (DataTable|GetDataTableRowNames "/Game/Main/RandomNFT/FData/DT_M_Head.DT_M_Head"))
      (bind _returnvalue_3 (Utilities|GetDataTableRow "/Game/Main/RandomNFT/FData/DT_M_Head.DT_M_Head" (Utilities|Array|Get(acopy) _outrownames_2 (Math|Random|RandomIntegerinRange 0 (Utilities|Array|Length _outrownames_2))))
        (:then
          (Components|SkeletalMesh|SetSkeletalMeshAsset _head (.SkeletalMesh (Utilities|Struct|BreakS_Head _returnvalue_3)))
          (for _array_element_2 (.MaterialNumber (Utilities|Struct|BreakS_Head _returnvalue_3))
            (bind _returnvalue_4 (Rendering|Material|CreateDynamicMaterialInstance _head _array_element_2 0 "None" :!class /Script/Engine.PrimitiveComponent))
            (for _index_2 (range 1 (Utilities|Array|Get(acopy) (.ColorCounts (Utilities|Struct|BreakS_Head _returnvalue_3)) _array_element_2))
              (bind _newparam_2 (CallFunction|RandomColor))
              (Rendering|Material|SetVectorParameterValue _returnvalue_4 (Utilities|String|StringToName (Utilities|String|Append "Color " (Utilities|String|ToString(Integer) _index_2))) _newparam_2 :!class /Script/Engine.MaterialInstanceDynamic)))
          (if (.IsHair (Utilities|Struct|BreakS_Head _returnvalue_3))
            (switch int (Math|Random|RandomIntegerinRange 0 1)
              (:0
                (CallFunction|CustomMesh "/Game/Main/RandomNFT/FData/DT_M_Hair.DT_M_Hair" (Variables|Default|GetHair)))
              (:1
                (CallFunction|CustomMesh "/Game/Main/RandomNFT/FData/DT_M_Hat.DT_M_Hat" (Variables|Default|GetHair))))
            (CallFunction|CustomMesh "/Game/Main/RandomNFT/FData/DT_M_Eyebrow.DT_M_Eyebrow" (Variables|Default|GetBeard))
            (CallFunction|CustomMesh "/Game/Main/RandomNFT/FData/DT_M_Beard.DT_M_Beard" (Variables|Default|GetEyebrow))
            (Components|StaticMesh|SetStaticMesh (Variables|Default|GetEyes) "/Game/StylizedModularChar/Meshes/SM_Eyes.SM_Eyes")))))))

(event Custom|ResetNFT
  (CallFunction|ClearSkMesh (Variables|Default|GetHead))
  (CallFunction|ClearMesh (Variables|Default|GetEyes))
  (CallFunction|ClearMesh (Variables|Default|GetHair))
  (CallFunction|ClearMesh (Variables|Default|GetEyebrow))
  (CallFunction|ClearMesh (Variables|Default|GetBeard))
  (Utilities|FlowControl|Delay 0.5)
  (CallFunction|CreateNFT)
  (Utilities|FlowControl|Delay 0.5)
  (CallFunction|ResultWidget)
  (Variables|Default|SetIsRandom false))

(event Custom|CustomMesh
  (params (Table :type Data%20Table%20Object%20Reference) (타깃 :type Static%20Mesh%20Component%20Object%20Reference))
  (bind _outrownames (DataTable|GetDataTableRowNames Table))
  (bind _returnvalue (Utilities|GetDataTableRow Table (Utilities|Array|Get(acopy) _outrownames (Math|Random|RandomIntegerinRange 0 (Utilities|Array|Length _outrownames))))
    (:then
      (Components|StaticMesh|SetStaticMesh 타깃 (.StaticMesh (Utilities|Struct|BreakS_CustomMesh _returnvalue)))
      (for _array_element (.MaterialNumber (Utilities|Struct|BreakS_CustomMesh _returnvalue))
        (bind _returnvalue_2 (Rendering|Material|CreateDynamicMaterialInstance 타깃 _array_element 0 "None" :!class /Script/Engine.PrimitiveComponent))
        (for _index (range 1 (Utilities|Array|Get(acopy) (.ColorCounts (Utilities|Struct|BreakS_CustomMesh _returnvalue)) _array_element))
          (bind _newparam (CallFunction|RandomColor))
          (Rendering|Material|SetVectorParameterValue _returnvalue_2 (Utilities|String|StringToName (Utilities|String|Append "Color " (Utilities|String|ToString(Integer) _index))) _newparam :!class /Script/Engine.MaterialInstanceDynamic))))))

(event Custom|CustomAnimation
  (params (Table :type Data%20Table%20Object%20Reference) (타깃 :type Static%20Mesh%20Component%20Object%20Reference))
  (bind _outrownames (DataTable|GetDataTableRowNames Table))
  (for _array_element _outrownames
    (bind _returnvalue (Utilities|GetDataTableRow Table _array_element)
      (:then
        (Components|StaticMesh|SetStaticMesh 타깃 (.StaticMesh (Utilities|Struct|BreakS_CustomMesh _returnvalue))))))
  (bind _returnvalue_2 (Utilities|GetDataTableRow Table (Utilities|Array|Get(acopy) _outrownames (Math|Random|RandomIntegerinRange 0 (Utilities|Array|Length _outrownames))))
    (:then
      (Components|StaticMesh|SetStaticMesh 타깃 (.StaticMesh (Utilities|Struct|BreakS_CustomMesh _returnvalue_2)))
      (for _array_element_2 (.MaterialNumber (Utilities|Struct|BreakS_CustomMesh _returnvalue_2))
        (Rendering|Material|CreateDynamicMaterialInstance 타깃 _array_element_2 0 "None" :!class /Script/Engine.PrimitiveComponent)))))

(event Custom|ClearMesh
  (params (타깃 :type Static%20Mesh%20Component%20Object%20Reference))
  (for (_ _array_index) (Rendering|Material|GetMaterials 타깃)
    (Rendering|Material|SetMaterial 타깃 _array_index 0)
    (Components|StaticMesh|SetStaticMesh 타깃 0)))

(event Custom|Clear%20SkMesh
  (params (타깃 :type Skeletal%20Mesh%20Component%20Object%20Reference))
  (for (_ _array_index) (Rendering|Material|GetMaterials 타깃)
    (Rendering|Material|SetMaterial 타깃 _array_index 0)
    (Components|SkeletalMesh|SetSkeletalMeshAsset 타깃 0)))

(event Custom|ResultWidget
  (bind _asbpw_nftresult (Utilities|Casting|CastToBPW_NFTResult (UserInterface|GetWidget (Variables|Default|GetWidget))))
  (Default|UpdateResult _asbpw_nftresult (Utilities|Text|ToText(String) (Utilities|GetObjectName (Components|SkeletalMesh|GetSkeletalMeshAsset (Variables|Default|GetHead)))) (Utilities|Text|ToText(String) (Utilities|GetObjectName (Variables|/Script/Engine.StaticMeshComponent|GetStaticMesh (Variables|Default|GetHair)))) (Utilities|Text|ToText(String) (Utilities|GetObjectName (Variables|/Script/Engine.StaticMeshComponent|GetStaticMesh (Variables|Default|GetEyebrow)))) (Utilities|Text|ToText(String) (Utilities|GetObjectName (Variables|/Script/Engine.StaticMeshComponent|GetStaticMesh (Variables|Default|GetBeard))))))

(event EventBeginPlay
  (bind _head (Variables|Default|GetHead))
  (Utilities|Array|Add (Variables|/Game/PhysicalS/BP/BP_Lever.BP_Lever_C|GetConnectedActors (.AsBP%20Lever (Utilities|Casting|CastToBP_Lever (Variables|/Script/Engine.ChildActorComponent|GetChildActor (Variables|Default|GetLever))))) self)
  (Transformation|AttachComponentToComponent (Variables|Default|GetEyes) _head "headSocket" "KeepRelative" "KeepRelative" "KeepRelative" true)
  (Transformation|AttachComponentToComponent (Variables|Default|GetEyebrow) _head "headSocket" "KeepRelative" "KeepRelative" "KeepRelative" true)
  (Transformation|AttachComponentToComponent (Variables|Default|GetHair) _head "headSocket" "KeepRelative" "KeepRelative" "KeepRelative" true)
  (Transformation|AttachComponentToComponent (Variables|Default|GetBeard) _head "headSocket" "KeepRelative" "KeepRelative" "KeepRelative" true))

(event EventDInteractFloat
  (params (Value :type Float%20%28double-precision%29) (Source :type Integer))
  (if (not (Variables|Default|GetIsRandom))
    (if (>= Value 7e+01)
      (Variables|Default|SetIsRandom true)
      (CallFunction|ResetNFT))))

(event EventDInteractBool
  (params (Value :type Boolean) (Source :type Integer)))

(event Input|KeyboardEvents|R
  (params (Key :type Key%20Structure :default "None"))
  (:Pressed
    (if (not (Variables|Default|GetIsRandom))
      (Variables|Default|SetIsRandom true)
      (CallFunction|ResetNFT))))

(fn ConstructionScript)

(fn RandomColor
  (return (Math|Color|MakeColor (Math|Random|RandomFloat) (Math|Random|RandomFloat) (Math|Random|RandomFloat))))