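; A bounce block actor, owned by a BP_BounceBlockPool, that rises and reddens according to how close an overlapping character is.
; While a character is inside its sphere, a throttled Tick converts distance from the block's start point into height and color values.
; Timelines scrubbed with SetNewTime lerp relative Z and a dynamic material's Base Color.
; Ending the overlap calls the Reverse events, which play those timelines.
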(event OnComponentBeginOverlap(Sphere)
  (params (OverlappedComponent :type Primitive%20Component%20Object%20Reference) (OtherActor :type Actor%20Object%20Reference) (OtherComp :type Primitive%20Component%20Object%20Reference) (OtherBodyIndex :type Integer) (bFromSweep :type Boolean) (SweepResult :type Hit%20Result%20Structure%20%28by%20ref%29))
  (bind _as캐릭터 (Utilities|Casting|CastToCharacter OtherActor))
  (Variables|Default|SetOverlapCharacter _as캐릭터)
  (if (not (Variables|Default|GetIsOverlap))
    (Variables|Default|SetIsOverlap true)))

(event OnComponentEndOverlap(Sphere)
  (params (OverlappedComponent :type Primitive%20Component%20Object%20Reference) (OtherActor :type Actor%20Object%20Reference) (OtherComp :type Primitive%20Component%20Object%20Reference) (OtherBodyIndex :type Integer))
  (bind _as캐릭터 (Utilities|Casting|CastToCharacter OtherActor))
  (if (Variables|Default|GetIsOverlap)
    (Variables|Default|SetIsOverlap false)
    (CallFunction|ReverseBounceBlockColor)
    (CallFunction|ReverseBounceBlockHeight)))

(event Custom|SetBounceBlockColor
  (params (In%20Color :type Linear%20Color%20Structure) (In%20Value :type Float%20%28double-precision%29) (In%20Time :type Float%20%28double-precision%29))
  (bind _alpha (Timeline|Curv SetNewTime)
    (:Update
      (Rendering|Material|SetVectorParameterValue (Variables|Default|GetBouncBlockMaterial) "Base Color" (Math|Color|MakeColor (Math|Float|Lerp 0.0 In%20Value _alpha) 0.0 0.0 (.A (Math|Color|BreakColor In%20Color))) :!class /Script/Engine.MaterialInstanceDynamic))))

(event Custom|SetBounceBlockHeight
  (params (InHeight :type Float%20%28double-precision%29) (inTime :type Float%20%28double-precision%29))
  (bind _initlocation (Variables|Default|GetInitLocation))
  (bind (_x _y _z) (Math|Vector|BreakVector _initlocation))
  (bind _alpha (Timeline|Cruv SetNewTime)
    (:Update
      (Transformation|SetActorRelativeLocation (Math|Vector|MakeVector _x _y (Math|Float|Lerp _z (+ _z InHeight) _alpha))))))

(event Custom|ReverseBounceBlockHeight
  (bind _initlocation (Variables|Default|GetInitLocation))
  (bind (_x _y _z) (Math|Vector|BreakVector _initlocation))
  (bind _alpha (Timeline|Cruv Play)
    (:Update
      (Transformation|SetActorRelativeLocation (Math|Vector|MakeVector _x _y (Math|Float|Lerp _z (+ _z (stale Custom|SetBounceBlockHeight InHeight)) _alpha))))))

(event Custom|ReverseBounceBlockColor
  (bind _alpha (Timeline|Curv Play)
    (:Update
      (Rendering|Material|SetVectorParameterValue (Variables|Default|GetBouncBlockMaterial) "Base Color" (Math|Color|MakeColor (Math|Float|Lerp 0.0 (stale Custom|SetBounceBlockColor In%20Value) _alpha) 0.0 0.0 (.A (Math|Color|BreakColor (stale Custom|SetBounceBlockColor In%20Color)))) :!class /Script/Engine.MaterialInstanceDynamic))))

(event EventBeginPlay
  (Utilities|FlowControl|Sequence
    (:then_0
      (Variables|Default|SetInitLocation (Transformation|GetActorLocation)))
    (:then_1
      (bind _returnvalue (Rendering|Material|CreateDynamicMaterialInstance (Variables|Default|GetBounceBlock) 0 0 "None" :!class /Script/Engine.PrimitiveComponent))
      (bind _output_get (Variables|Default|SetBouncBlockMaterial _returnvalue))
      (bind _returnvalue_2 (Rendering|Material|GetVectorParameterValue _output_get "Base Color" :!class /Script/Engine.MaterialInstanceDynamic))
      (Variables|Default|SetInitColor _returnvalue_2))
    (:then_2
      (bind _asbp_bounce_block_pool (Utilities|Casting|CastToBP_BounceBlockPool (Components|GetOwner)))
      (Variables|Default|SetBounceBlockPool _asbp_bounce_block_pool))))

(event EventTick
  (params (DeltaSeconds :type Float%20%28single-precision%29))
  (bind _initlocation (Variables|Default|GetInitLocation))
  (bind _overlapcharacter (Variables|Default|GetOverlapCharacter))
  (bind _returnvalue (Transformation|GetActorLocation _overlapcharacter))
  (bind _capsulecomponent (Variables|/Script/Engine.Character|GetCapsuleComponent _overlapcharacter))
  (bind _returnvalue_2 (Components|Capsule|GetScaledCapsuleHalfHeight _capsulecomponent))
  (bind _returnvalue_3 (+ (.z _initlocation) _returnvalue_2))
  (bind _returnvalue_4 (Math|Vector|Distance(Vector) (Math|Vector|MakeVector (.x _initlocation) (.y _initlocation) _returnvalue_3) _returnvalue))
  (bind _returnvalue_5 (/ _returnvalue_4 5e+01))
  (bind _returnvalue_6 (Math|Float|Clamp(Float) _returnvalue_5 0.0 1e+01))
  (if (Variables|Default|GetIsOverlap)
    (bind _output_get (Variables|Default|SetdelayTime (- (Variables|Default|GetdelayTime) DeltaSeconds)))
    (if (<= _output_get 0.0)
      (Variables|Default|SetdelayTime 0.05)
      (Utilities|IsValid _overlapcharacter
        (:Is%20Valid
          (CallFunction|SetBounceBlockHeight (* (- 1e+01 _returnvalue_6) 5.0) (/ _returnvalue_6 2e+01))
          (CallFunction|SetBounceBlockColor "(R=50.000000,G=0.000000,B=0.000000,A=1.000000)" (- 1.0 (/ _returnvalue_6 1e+01)) (- _returnvalue_6 1e+01)))))))

(fn ConstructionScript)