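; Teleport trigger actor that moves an overlapping VoiceChatCharacter into a multiplayer session as host or client.
; Box overlap reads the character's IsServer flag to choose between hosting and joining.
; With LAN set, the host creates a two-connection session and opens TravelLevel as listen server, while clients join the first session found.
; Without LAN, console open commands either host TravelLevel or connect to ServerIP.
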(event OnComponentBeginOverlap(Box)
  (params (OverlappedComponent :type Primitive%20Component%20Object%20Reference) (OtherActor :type Actor%20Object%20Reference) (OtherComp :type Primitive%20Component%20Object%20Reference) (OtherBodyIndex :type Integer) (bFromSweep :type Boolean) (SweepResult :type Hit%20Result%20Structure%20%28by%20ref%29))
  (bind _asvoice_chat_character (Utilities|Casting|CastToVoiceChatCharacter OtherActor))
  (Variables|Default|SetAs%20Voice%20Chat%20Character _asvoice_chat_character)
  (if (Variables|/Game/Main/VoicChat/VoiceChatCharacter.VoiceChatCharacter_C|GetIsServer _asvoice_chat_character)
    (bind _as플레이어_컨트롤러 (Utilities|Casting|CastToPlayerController (Pawn|GetController (Variables|Default|GetAs%20Voice%20Chat%20Character))))
    (if (Variables|Default|GetLAN)
      (|Session _as플레이어_컨트롤러 2 true
        (:OnSuccess
          (Game|OpenLevel(byName) (Utilities|String|StringToName (Variables|Default|GetTravelLevel)) true "?listen")))
      (else
        (Development|ExecuteConsoleCommand (Utilities|String|Append "open " (Variables|Default|GetTravelLevel) "?listen") _as플레이어_컨트롤러)))
    (else
      (bind _as플레이어_컨트롤러_2 (Utilities|Casting|CastToPlayerController (Pawn|GetController (Variables|Default|GetAs%20Voice%20Chat%20Character))))
      (if (Variables|Default|GetLAN)
        (bind _results (|FindSessions _as플레이어_컨트롤러_2 1 (Variables|Default|GetLAN))
          (:OnSuccess
            (|JoinSession _as플레이어_컨트롤러_2 (Utilities|Array|Get(acopy) _results))))
        (else
          (Development|ExecuteConsoleCommand (Utilities|String|Append "open" (Variables|Default|GetServerIP)) _as플레이어_컨트롤러_2))))))

(event EventBeginPlay)

(event Collision|EventActorBeginOverlap
  (params (OtherActor :type Actor%20Object%20Reference)))

(event EventTick
  (params (DeltaSeconds :type Float%20%28single-precision%29)))

(fn ConstructionScript)